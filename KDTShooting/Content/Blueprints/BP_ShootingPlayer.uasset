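; BP_ShootingPlayer is a player Blueprint that, as it stands, only exercises test functions and prints their results.
; On BeginPlay it calls AddTest and Multiply on fixed inputs, prints both along with GetNumberFloat and GetLocationVector, then calls PrintInputNumber.
; Those functions are defined outside this file; overlap, Tick and the construction script do nothing.
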(event EventBeginPlay
  (bind _self self)
  (bind _returnvalue (Class|ShootingPlayer|AddTest _self 5 11))
  (Development|PrintString (Utilities|String|ToString(Integer) _returnvalue))
  (bind _returnvalue_2 (Class|ShootingPlayer|Multiply _self 5 11))
  (Development|PrintString (Utilities|String|ToString(Integer) _returnvalue_2))
  (Development|PrintString (Utilities|String|ToString(Float) (Class|ShootingPlayer|GetNumberFloat _self)))
  (Development|PrintString (Utilities|String|ToString(Vector) (Class|ShootingPlayer|GetLocationVector _self)))
  (Class|ShootingPlayer|PrintInputNumber 10))

(event Collision|EventActorBeginOverlap
  (params (OtherActor :type Actor%20Object%20Reference)))

(event EventTick
  (params (DeltaSeconds :type Float%20%28single-precision%29)))

(fn ConstructionScript)